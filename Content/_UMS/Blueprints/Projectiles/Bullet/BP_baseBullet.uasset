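; Base bullet projectile that plays an explosion sound and emitter on spawn, then handles damage and impact effects on hit.
; A Box hit fires a radial impulse, applies damage credited to the player character, and branches on the hit actor's Metal or Flesh tag for emitters.
; Flesh hits call AnyDamage on player or AI characters; AI hits also notify the game mode via EnemyGameEnded and start BP_SlowMotionController's slow motion.
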(event OnComponentHit(Box)
  (params (HitComponent :type Primitive%20Component%20Object%20Reference) (OtherActor :type Actor%20Object%20Reference) (OtherComp :type Primitive%20Component%20Object%20Reference) (NormalImpulse :type Vector :default "0, 0, 0") (Hit :type Hit%20Result%20Structure%20%28by%20ref%29))
  (bind (_bblockinghit _binitialoverlap _time _distance _location _impactpoint _normal _impactnormal _physmat _hitactor) (Collision|BreakHitResult Hit))
  (Variables|Default|SetOther%20Actor OtherActor)
  (Class|RadialForceComponent|FireImpulse (Variables|Default|GetRadialForce))
  (Variables|Default|SetHitLocation _location)
  (Effects|SpawnEmitteratLocation 0 _location)
  (Audio|PlaySoundatLocation 0 _location "0, 0, 0" 1.0 1.0 0.0 0 0 0 0)
  (Game|Damage|ApplyDamage _hitactor (Variables|Default|GetBase%20Damage) 0 (Game|GetPlayerCharacter 0))
  (Utilities|IsValid _hitactor
    (:Is%20Valid
      (if (Actor|ActorHasTag _hitactor "Metal")
        ;[0.15 0.15 0.15 0.5] Metal
        (Effects|SpawnEmitteratLocation 0 (Variables|Default|GetHitLocation))
        (Development|PrintString "Metal Hit")
        (Actor|DestroyActor)
        (elif (Actor|ActorHasTag _hitactor "Flesh")
          ;[0.15 0.15 0.15 0.5] Flesh
          (Effects|SpawnEmitteratLocation 0 (Variables|Default|GetHitLocation))
          (Development|PrintString "FLESH")
          (bind _asbp_third_person_character (Utilities|Casting|CastToBP_ThirdPersonCharacter (Variables|Default|GetOther%20Actor))
            (:then
              (Default|AnyDamage _asbp_third_person_character)
              ;[0.15 0.15 0.15 0.5] s 1.6
              (Actor|DestroyActor :!label _label))
            (:CastFailed
              (bind _asbp_base_ai_character (Utilities|Casting|CastToBP_Base_AI_Character (Variables|Default|GetOther%20Actor))
                (:then
                  (Default|AnyDamage _asbp_base_ai_character)
                  (bind _asbp_game_mode_base (Utilities|Casting|CastToBP_GameModeBase (Game|GetGameMode))
                    (:then
                      (Default|EnemyGameEnded _asbp_game_mode_base)
                      (bind _outactors (Actor|GetAllActorsOfClass "/Game/_UMS/Blueprints/Effects/BP_SlowMotionController.BP_SlowMotionController_C"))
                      (Development|PrintString (Utilities|GetDisplayName (Utilities|Array|Get(acopy) _outactors)))
                      (Development|PrintString "Attempted to slow motion")
                      (Default|StartSlowMotion (Utilities|Array|Get(acopy) _outactors))
                      (goto _label))
                    (:CastFailed
                      (Development|PrintString "BP_GameModeBase CAST FAILED"))))
                (:CastFailed
                  (Development|PrintString "Cast to BP_Base_AI_CHARACTER FAILED")))))
          (else
            ;[0.15 0.15 0.15 0.5] Other
            (Effects|SpawnEmitteratLocation 0 (Variables|Default|GetHitLocation))
            (Actor|DestroyActor)))))))

(event EventBeginPlay
  (bind _returnvalue (Transformation|GetActorLocation))
  (Audio|PlaySoundatLocation "/Game/StarterContent/Audio/Explosion01.Explosion01" _returnvalue "0, 0, 0" 1.0 1.0 0.0 0 0 0 0)
  (Effects|SpawnEmitteratLocation 0 _returnvalue))

(event Collision|EventActorBeginOverlap
  (params (OtherActor :type Actor%20Object%20Reference)))

(event EventTick
  (params (DeltaSeconds :type Float%20%28single-precision%29)))

(fn ConstructionScript)