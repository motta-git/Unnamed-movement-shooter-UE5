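; Base game mode that advances the game to the next level once all enemies in the current one are gone.
; BeginPlay counts BP_Base_AI_Character actors, and each EnemyGameEnded call decrements that count.
; At zero or below, after a short delay, it increments CurrentLevelIndex on BP_GameInstance and opens that entry in LevelOrder.
; ChangeToNextLevel performs the same index-based switch immediately, and debug prints trace the flow.
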(event Custom|EnemyGameEnded
  (bind _output_get (Variables|Default|SetenemyCount (- (Variables|Default|GetenemyCount) 1)))
  (Development|PrintString "Enemies remaining:")
  (Development|PrintString (Utilities|String|ToString(Integer) _output_get))
  (Math|Integer|CompareInt _output_get
    (:==
      _)
    (:<
      _))
  (Utilities|FlowControl|Delay 1.0)
  (bind _asbp_game_instance (Utilities|Casting|CastToBP_GameInstance (Game|GetGameInstance)))
  (bind _output_get_2 (Variables|/Game/_UMS/Blueprints/Gamemode/BP_GameInstance.BP_GameInstance_C|SetcurrentLevelIndex _asbp_game_instance (+ (Variables|/Game/_UMS/Blueprints/Gamemode/BP_GameInstance.BP_GameInstance_C|GetcurrentLevelIndex _asbp_game_instance) 1)))
  (Game|OpenLevel(byName) (Utilities|Array|Get(acopy) (Variables|Default|GetlevelOrder) _output_get_2))
  (Development|PrintString (Utilities|String|ToString(Name) (Utilities|Array|Get(acopy) (Variables|Default|GetlevelOrder) _output_get_2))))

(event EventBeginPlay
  (bind _outactors (Actor|GetAllActorsOfClass "/Game/_UMS/Blueprints/Characters/AI/BP_Base_AI_Character.BP_Base_AI_Character_C"))
  (bind _output_get (Variables|Default|SetenemyCount (Utilities|Array|Length _outactors)))
  (Development|PrintString (Utilities|String|ToString(Integer) _output_get))
  (Development|PrintString "Gamemode loaded OK!")
  (bind _returnvalue (Game|GetCurrentLevelName true))
  (Variables|Default|SetcurrentLevelName _returnvalue))

(event EventTick
  (params (DeltaSeconds :type Float%20%28single-precision%29)))

(fn ConstructionScript)

(fn ChangetoNextLevel
  (bind _asbp_game_instance (Utilities|Casting|CastToBP_GameInstance (Game|GetGameInstance)))
  (bind _output_get (Variables|/Game/_UMS/Blueprints/Gamemode/BP_GameInstance.BP_GameInstance_C|SetcurrentLevelIndex _asbp_game_instance (+ (Variables|/Game/_UMS/Blueprints/Gamemode/BP_GameInstance.BP_GameInstance_C|GetcurrentLevelIndex _asbp_game_instance) 1)))
  (Game|OpenLevel(byName) (Utilities|Array|Get(acopy) (Variables|Default|GetlevelOrder) _output_get))
  (Development|PrintString "Hello"))