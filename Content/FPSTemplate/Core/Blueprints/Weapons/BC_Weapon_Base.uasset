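; Base weapon actor for the FPS template, with a skeletal mesh and a flag for whether someone is holding it.
; On BeginPlay, a held weapon turns off physics simulation and mesh collision.
; A setter updates the held flag without reapplying physics, and the nodes that would enable physics with PhysicsActor collision are not connected.
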(event EventBeginPlay
  (if (Variables|Default|GetisBeingHeldBySomeone?)
    (Physics|SetSimulatePhysics (Variables|Default|GetSkeletalMesh) false)
    (Collision|SetCollisionProfileName (Variables|Default|GetSkeletalMesh) "NoCollision" true :!class /Script/Engine.PrimitiveComponent)))

(event Collision|EventActorBeginOverlap
  (params (OtherActor :type Actor%20Object%20Reference)))

(event EventTick
  (params (DeltaSeconds :type Float%20%28single-precision%29)))

(fn ConstructionScript)

(fn SetIsBeingHeldbySomeone
  (params (bool :type Boolean))
  (Variables|Default|SetisBeingHeldBySomeone? bool))